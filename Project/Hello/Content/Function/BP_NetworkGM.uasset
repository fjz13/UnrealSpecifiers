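; BP_NetworkGM is a network game mode that numbers player controllers as they join.
; On PostLogin it casts the new player to BP_NetworkPC, copies its running Index counter onto that controller, then increments the counter.
; Unconnected leftover nodes for a delayed, authority-only BP_Network spawn and a login debug print never run.
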(event `self.ReceiveBeginPlay`)

(event `self.K2_PostLogin`
  (params (NewPlayer :type "PlayerController Object Reference"))
  (bind _asbp_network_pc (cast `/Game/Function/BP_NetworkPC` NewPlayer))
  (set `/Game/Function/BP_NetworkPC.Index` (`self.Index`) _asbp_network_pc)
  (`/Engine/EditorBlueprintResources/StandardMacros.IncrementInt` (`self.Index`)))

(fn `UserConstructionScript`)