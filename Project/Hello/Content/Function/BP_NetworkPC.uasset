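; BP_NetworkPC is a test Blueprint, apparently a player controller, for exercising network RPC and C++ event functions.
; OtherClientFunc and OtherServerFunc report their status through InsiderSubsystem's PrintFuncStatus.
; BeginPlay only delays into an authority switch with no connected outputs; the other client/server test calls are disconnected and never run.
; The implementable event prints "PC", while the native event override is empty.
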(event `OtherClientFunc`
  (`InsiderSubsystem.PrintFuncStatus` (subsystem `InsiderSubsystem`) self "OtherClientFunc"))

(event `self.ReceiveBeginPlay`
  (`KismetSystemLibrary.Delay` 5.0)
  (`/Engine/EditorBlueprintResources/ActorMacros.Switch Has Authority`))

(event `OtherServerFunc`
  (`InsiderSubsystem.PrintFuncStatus` (subsystem `InsiderSubsystem`) self "OtherServerFunc"))

(fn `Func_ImplementableEvent`
  (`KismetSystemLibrary.PrintString` "PC"))

(fn `Func_NativeEvent`)

(fn `UserConstructionScript`)