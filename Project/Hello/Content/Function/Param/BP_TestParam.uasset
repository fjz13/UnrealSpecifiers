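; BP_TestParam is a test Blueprint that exercises function parameter variants: const and non-const, by value, reference or out, required, display name and defaults.
; On BeginPlay it calls MyFuncTestParamNoConstStruct and sets MyInt on the returned struct by reference.
; The other test calls, including a print sequence comparing copy and reference passing, are not connected to any event.
; NewFunction is a stub returning empty values.
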(event `self.ReceiveBeginPlay`
  (bind _mystruct (`self.MyFuncTestParam_NoConstStruct`))
  (setmembers `MyCommonStruct` :`StructRef` _mystruct :`MyInt` 123))

(fn `NewFunction`
  (params (NewParam :type String) (NewParam2 :type Integer))
  (returns (NewParam1 :type String) (NewParam3 :type "Vector Structure"))
  (return "" (0.0 0.0 0.0)))

(fn `UserConstructionScript`)